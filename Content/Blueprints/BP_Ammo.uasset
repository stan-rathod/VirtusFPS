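; BP_Ammo is an ammo pickup that refills the reserve of the player's primary weapon.
; When BP_Player overlaps it, it raises PrimaryWeaponBP's MaxAmmo by a fixed amount up to a cap, then destroys itself with a particle and sound effect.
; Tick spins the pickup by a fixed yaw each frame and plays the Ammo timeline, whose track moves it by a local offset.
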(event `self.ReceiveActorBeginOverlap`
  (params (OtherActor :type "Actor Object Reference"))
  (bind _returnvalue (`self.K2_GetActorLocation`))
  (bind _asbp_player (cast `/Game/Blueprints/BP_Player` OtherActor))
  (bind _primaryweaponbp (`/Game/Blueprints/BP_Player.PrimaryWeaponBP` _asbp_player))
  (bind _maxammo (`/Game/Weapons/AK47/BP_Weapon_AK47.MaxAmmo` _primaryweaponbp))
  (if (<= _maxammo 330)
    (set `/Game/Weapons/AK47/BP_Weapon_AK47.MaxAmmo` (+ _maxammo 30) _primaryweaponbp)
    (else
      (set `/Game/Weapons/AK47/BP_Weapon_AK47.MaxAmmo` 360 _primaryweaponbp)))
  (`self.K2_DestroyActor`)
  (`GameplayStatics.SpawnEmitterAtLocation` "/Game/Effects/Pickups/Particles/P_Collectable.P_Collectable" _returnvalue)
  (`GameplayStatics.SpawnSoundAtLocation` "/Game/Audio/A_Powerup.A_Powerup" _returnvalue (struct) 0.3 1.0 0.0 null null))

(event `self.ReceiveTick`
  (params (DeltaSeconds :type "Float (single-precision)"))
  (`self.K2_AddActorLocalRotation` (struct :`Yaw` 3.0))
  (bind (_direction _newtrack_0) (`Timeline|Ammo`)
    (:`Update`
      (`self.K2_AddActorLocalOffset` _newtrack_0))))

(fn `UserConstructionScript`)