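; Enemy AI pawn that wanders between random reachable points and damages BP_Player on contact during timed attack windows.
; Seeing the player starts another move, though without a destination set, and SeenPlayer stays false so roaming never stops.
; Each successful move opens a brief attack window in which sphere overlap can hit once, then repeats.
; Hit reaction, health loss and death with killfeed are present but unconnected.
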(event `self.ReceiveBeginPlay`
  (`|AIMoveTo` self (`NavigationSystemV1.K2_GetRandomReachablePointInRadius` (`self.K2_GetActorLocation`) 10000.0 null null) null :!label _label
    (:`OnSuccess`
      _)
    (:`OnFail`
      _))
  (if (not (`self.seenPlayer`))
    (goto _label)))

(event `self.ReceiveActorBeginOverlap`
  (params (OtherActor :type "Actor Object Reference")))

(event `self.PawnSensing.OnSeePawn`
  (params (Pawn :type "Pawn Object Reference"))
  (bind _asbp_player (cast `/Game/Blueprints/BP_Player` Pawn))
  (set `self.seenPlayer` false)
  (`|AIMoveTo` _asbp_player self (0.0 0.0 0.0) null :!label _label_2
    (:`OnSuccess`
      (if (not (`self.canAttack`))
        (set `self.canAttack` true)
        (`KismetSystemLibrary.Delay` 2.3)
        (set `self.canAttack` false)
        (set `self.alreadyHitPlayer` false)
        (goto _label_2)))))

(event `self.Sphere.OnComponentBeginOverlap`
  (params (OverlappedComponent :type "PrimitiveComponent Object Reference") (OtherActor :type "Actor Object Reference") (OtherComp :type "PrimitiveComponent Object Reference") (OtherBodyIndex :type Integer) (bFromSweep :type Boolean) (SweepResult :type "HitResult Structure (by ref)"))
  (bind _asbp_player (cast `/Game/Blueprints/BP_Player` OtherActor))
  (if (`self.canAttack`)
    (if (not (`self.alreadyHitPlayer`))
      (`/Game/Blueprints/BP_Player.TakeDamage5%` _asbp_player)
      (set `self.alreadyHitPlayer` true))))

(fn `UserConstructionScript`)