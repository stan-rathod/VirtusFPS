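; AK47 weapon Blueprint that handles hitscan firing and reloading for the player.
; Fire line-traces from the aim or hip first-person camera, spends ammo and spawns a muzzle effect at the primary weapon's socket.
; Hits on BP_EnemyAI show a hit marker and deduct health, spawning blood or, at zero health, enabling ragdoll physics and a killfeed widget.
; Reload refills the clip from reserve ammo and flags the player as reloading.
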(event `self.ReceiveBeginPlay`
  (bind _asbp_player (cast `/Game/Blueprints/BP_Player` (`GameplayStatics.GetPlayerCharacter` 0)))
  (set `self.Player` _asbp_player))

(event `Fire`
  (bind _firstpersoncamera (`/Game/Blueprints/BP_Player.FirstPersonCamera` (`self.Player`)))
  (bind _firstpersonaimcamera (`/Game/Blueprints/BP_Player.FirstPersonAimCamera` (`self.Player`)))
  (bind _returnvalue (`SceneComponent.K2_GetComponentLocation` _firstpersoncamera))
  (bind _returnvalue_2 (`SceneComponent.K2_GetComponentLocation` _firstpersonaimcamera))
  (bind _weaponmesh (`/Game/Weapons/AK47/BP_Weapon_AK47.WeaponMesh` (`/Game/Blueprints/BP_Player.PrimaryWeaponBP` (`self.Player`))))
  (bind _weaponmesh_2 (`/Game/Weapons/AK47/BP_Weapon_AK47.WeaponMesh` (`/Game/Blueprints/BP_Player.PrimaryWeaponBP` (`self.Player`))))
  (if (`/Game/Blueprints/BP_Player.isInAiming` (`self.Player`))
    (bind _outhit (`KismetSystemLibrary.LineTraceSingle` _returnvalue_2 (+ _returnvalue_2 (* (`KismetMathLibrary.GetForwardVector` (`SceneComponent.K2_GetComponentRotation` _firstpersonaimcamera)) 1500.0)) "TraceTypeQuery1"))
    (set `self.Ammo` (- (`self.Ammo`) 1))
    (`GameplayStatics.SpawnEmitterAtLocation` "/Game/Effects/GenericImpact/P_RifleImpact.P_RifleImpact" (`SceneComponent.GetSocketLocation` _weaponmesh "Muzzle") (`SceneComponent.GetSocketRotation` _weaponmesh "Muzzle"))
    (bind (_bblockinghit _binitialoverlap _time _distance _location _impactpoint _normal _impactnormal _physmat _hitactor) (`GameplayStatics.BreakHitResult` _outhit))
    (bind _asbp_enemy_ai (cast `/Game/Blueprints/BP_EnemyAI` _hitactor))
    (bind _returnvalue_3 (`|CreateWidget` "/Game/UMG/WB_HitMarker.WB_HitMarker_C"))
    (`UserWidget.AddToViewport` _returnvalue_3 0)
    (bind _output_get (set `/Game/Blueprints/BP_EnemyAI.Health` (- (`/Game/Blueprints/BP_EnemyAI.Health` _asbp_enemy_ai) 0.2) _asbp_enemy_ai))
    (if (<= _output_get 0.0)
      (`PrimitiveComponent.SetSimulatePhysics` (`Character.Mesh` _asbp_enemy_ai) true)
      (bind _returnvalue_4 (`|CreateWidget` "/Game/UMG/WB_Killfeed.WB_Killfeed_C"))
      (`UserWidget.AddToViewport` _returnvalue_4 0)
      (else
        (`GameplayStatics.SpawnEmitterAtLocation` "/Game/Effects/BloodImpact/P_blood_splash_02.P_blood_splash_02" _location)))
    (else
      (bind _outhit_2 (`KismetSystemLibrary.LineTraceSingle` _returnvalue (+ _returnvalue (* (`KismetMathLibrary.GetForwardVector` (`SceneComponent.K2_GetComponentRotation` _firstpersoncamera)) 1500.0)) "TraceTypeQuery1"))
      (set `self.Ammo` (- (`self.Ammo`) 1))
      (`GameplayStatics.SpawnEmitterAtLocation` "/Game/Effects/GenericImpact/P_RifleImpact.P_RifleImpact" (`SceneComponent.GetSocketLocation` _weaponmesh_2 "Muzzle") (`SceneComponent.GetSocketRotation` _weaponmesh_2 "Muzzle"))
      (bind (_bblockinghit_2 _binitialoverlap_2 _time_2 _distance_2 _location_2 _impactpoint_2 _normal_2 _impactnormal_2 _physmat_2 _hitactor_2) (`GameplayStatics.BreakHitResult` _outhit_2))
      (bind _asbp_enemy_ai_2 (cast `/Game/Blueprints/BP_EnemyAI` _hitactor_2))
      (bind _returnvalue_5 (`|CreateWidget` "/Game/UMG/WB_HitMarker.WB_HitMarker_C"))
      (`UserWidget.AddToViewport` _returnvalue_5 0)
      (bind _output_get_2 (set `/Game/Blueprints/BP_EnemyAI.Health` (- (`/Game/Blueprints/BP_EnemyAI.Health` _asbp_enemy_ai_2) 0.2) _asbp_enemy_ai_2))
      (if (<= _output_get_2 0.0)
        (`PrimitiveComponent.SetSimulatePhysics` (`Character.Mesh` _asbp_enemy_ai_2) true)
        (bind _returnvalue_6 (`|CreateWidget` "/Game/UMG/WB_Killfeed.WB_Killfeed_C"))
        (`UserWidget.AddToViewport` _returnvalue_6 0)
        (else
          (`GameplayStatics.SpawnEmitterAtLocation` "/Game/Effects/BloodImpact/P_blood_splash_02.P_blood_splash_02" _location_2))))))

(fn `Reload`
  (returns (Output_Get :type Boolean) (Output_Get1 :type Boolean))
  (bind _returnvalue (- (`self.ClipAmmo`) (`self.Ammo`)))
  (if (< (`self.Ammo`) (`self.ClipAmmo`))
    (if (> (`self.MaxAmmo`) _returnvalue)
      (set `self.ExistingAmmo` _returnvalue)
      (set `self.Ammo` (+ (`self.Ammo`) (`self.ExistingAmmo`)))
      (set `self.MaxAmmo` (- (`self.MaxAmmo`) (`self.ExistingAmmo`)))
      (bind _output_get (set `/Game/Blueprints/BP_Player.isInReloading` true (`self.Player`)))
      (else
        (set `self.ExistingAmmo` _returnvalue)
        (set `self.Ammo` (+ (`self.Ammo`) (`self.MaxAmmo`)))
        (set `self.MaxAmmo` 0)
        (bind _output_get_2 (set `/Game/Blueprints/BP_Player.isInReloading` true (`self.Player`)))))
    (return _output_get _output_get_2)))

(fn `UserConstructionScript`)